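; BP_LobbyPC is a lobby player controller that relays chat messages between the player and the lobby game mode.
; It stores a player name through ChangeName, prefixes it to each outgoing message and passes the result to BP_LobbyGM.CatchPlayerMessage.
; ServerSendMessage receives a message and writes it to the BP_Hud UI text box, replacing the previous text.
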(event `ChangeName`
  (params (name :type Text))
  (set `self.Name` name))

(event `CatchOwnPlayerMessage`
  (params (CatchedMessage :type Text))
  (bind _asbp_lobby_gm (cast `/Game/Blueprints/BP_LobbyGM` (`GameplayStatics.GetGameMode`)))
  (`/Game/Blueprints/BP_LobbyGM.CatchPlayerMessage` _asbp_lobby_gm (`KismetTextLibrary.Conv_StringToText` (`KismetStringLibrary.Concat_StrStr` (`KismetTextLibrary.Conv_TextToString` (`self.Name`)) ": " (`KismetTextLibrary.Conv_TextToString` CatchedMessage)))))

(event `ServerSendMessage`
  (params (ServerMessage :type Text))
  (bind _asbp_hud (cast `/Game/Blueprints/BP_Hud` (`self.GetHUD`)))
  (set `TextBlock.Text` ServerMessage (`/Game/UI/WBP_UI.tbx_GetMessage` (`/Game/Blueprints/BP_Hud.UI` _asbp_hud))))

(fn `UserConstructionScript`)