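; Enemy spawner actor that periodically spawns BP_Enemy AI at its own location while player characters are within its spawn radius.
; An overlap with BP_ThirdPersonCharacter sets an in-radius flag, which lets the server-only Tick accumulate a timer.
; When the timer exceeds SpawnTimer, it spawns an enemy and restarts; once no character overlaps the radius, it clears the flag and timer.
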(event `self.ReceiveTick`
  (params (DeltaSeconds :type "Float (single-precision)"))
  (`/Engine/EditorBlueprintResources/ActorMacros.Switch Has Authority`
    (:`Authority`
      (if (`self.IsInRadius`)
        (if (> (`KismetArrayLibrary.Array_Length` (`PrimitiveComponent.GetOverlappingActors` (`self.SpawnRadius`) "/Game/ThirdPerson/Blueprints/BP_ThirdPersonCharacter.BP_ThirdPersonCharacter_C")) 0)
          (set `self.CurrentTimer` (+ DeltaSeconds (`self.CurrentTimer`)))
          ;[1 1 1] Timer fertig
          (if (< (`self.SpawnTimer`) (`self.CurrentTimer`))
            (set `self.CurrentTimer` 0.0)
            (`self.Spawn Enemys`)
            (`KismetSystemLibrary.PrintString` "Hello"))
          (else
            (set `self.IsInRadius` false)
            (set `self.CurrentTimer` 0.0)))))))

(event `self.SpawnRadius.OnComponentBeginOverlap`
  (params (OverlappedComponent :type "PrimitiveComponent Object Reference") (OtherActor :type "Actor Object Reference") (OtherComp :type "PrimitiveComponent Object Reference") (OtherBodyIndex :type Integer) (bFromSweep :type Boolean) (SweepResult :type "HitResult Structure (by ref)"))
  (cast `/Game/ThirdPerson/Blueprints/BP_ThirdPersonCharacter` OtherActor)
  (set `self.IsInRadius` true))

(fn `Spawn Enemys`
  (`AIBlueprintHelperLibrary.SpawnAIFromClass` "/Game/Blueprints/BP_Enemy.BP_Enemy_C" null (`self.K2_GetActorLocation`) (struct) false null))

(fn `UserConstructionScript`)