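; BP_Enemy is a networked suicide enemy that chases a randomly chosen third-person character and damages it by exploding on contact.
; Server-side Tick drives movement and re-picks the target when the enemy seems stalled, showing a spinning confusion text.
; Explode unregisters from its spawner, spawns an effect and flags nearby enemies to explode on their timers, creating chain reactions.
; Projectile overlap destroys it without exploding, while Health's OnRep triggers Explode below one.
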(event `self.ReceiveBeginPlay`
  (`self.Choose Player`)
  (`GameplayStatics.PlaySoundAtLocation` (`self.SpawnSound`) (`SceneComponent.K2_GetComponentLocation` (`self.Sphere`)) (struct) 1.0 1.0 0.0 null null null null))

(event `self.ReceiveTick`
  (params (DeltaSeconds :type "Float (single-precision)"))
  (bind (_returnvalue_x _returnvalue_y) (`KismetMathLibrary.BreakVector` (`self.GetVelocity`)))
  (bind _textrender (`self.TextRender`))
  (bind _textrender_2 (`self.TextRender`))
  (bind (_returnvalue_roll _returnvalue_pitch _returnvalue_yaw) (`KismetMathLibrary.BreakRotator` (`SceneComponent.K2_GetComponentRotation` _textrender_2)))
  (`/Engine/EditorBlueprintResources/ActorMacros.Switch Has Authority`
    (:`Authority`
      (`|ExecutionSequence`
        (:`then_0`
          (`AIBlueprintHelperLibrary.SimpleMoveToLocation` (`self.GetController`) (`self.K2_GetActorLocation` (`self.FollowingPlayer`))))
        (:`then_1`
          (if (`self.HasToExplode`)
            (bind _output_get (set `self.ExplodeTimer` (- (`self.ExplodeTimer`) DeltaSeconds)))
            (if (<= _output_get 0.0)
              (`self.Explode`))))
        (:`then_2`
          (if (and (<= _returnvalue_x 0.0) (<= _returnvalue_y 0.0))
            (bind _output_get_2 (set `self.CurrentVerwirrtTimer` (+ (`self.CurrentVerwirrtTimer`) DeltaSeconds)))
            (`SceneComponent.SetVisibility` _textrender true false)
            (if (>= _output_get_2 (`self.VerwirrtTimer`))
              (`self.Choose Player`)
              (set `self.CurrentVerwirrtTimer` 0.0))
            (else
              (set `self.CurrentVerwirrtTimer` 0.0)
              (`SceneComponent.SetVisibility` _textrender false false))))
        (:`then_3`
          (`SceneComponent.K2_SetWorldRotation` _textrender_2 (`KismetMathLibrary.MakeRotator` 0.0 0.0 (+ _returnvalue_yaw (* DeltaSeconds 125.0))) false false))))))

(event `self.ExplosionRadius.OnComponentBeginOverlap`
  (params (OverlappedComponent :type "PrimitiveComponent Object Reference") (OtherActor :type "Actor Object Reference") (OtherComp :type "PrimitiveComponent Object Reference") (OtherBodyIndex :type Integer) (bFromSweep :type Boolean) (SweepResult :type "HitResult Structure (by ref)"))
  (`/Engine/EditorBlueprintResources/ActorMacros.Switch Has Authority`
    (:`Authority`
      (bind _asbp_third_person_character (cast `/Game/ThirdPerson/Blueprints/BP_ThirdPersonCharacter` OtherActor))
      (`/Game/ThirdPerson/Blueprints/BP_ThirdPersonCharacter.GetDamage` _asbp_third_person_character (`self.ExplodeDamage`))
      (`self.Explode`))))

(event `self.Sphere.OnComponentBeginOverlap`
  (params (OverlappedComponent :type "PrimitiveComponent Object Reference") (OtherActor :type "Actor Object Reference") (OtherComp :type "PrimitiveComponent Object Reference") (OtherBodyIndex :type Integer) (bFromSweep :type Boolean) (SweepResult :type "HitResult Structure (by ref)"))
  (cast `/Game/Blueprints/BP_Projecttile` OtherActor)
  (`/Engine/EditorBlueprintResources/ActorMacros.Switch Has Authority`
    (:`Authority`
      (`self.K2_DestroyActor`))))

(event `OnProjectileHit`
  (params (Damage :type Integer))
  (`/Engine/EditorBlueprintResources/ActorMacros.Switch Has Authority`
    (:`Authority`
      (set `self.Health` (- (`self.Health`) Damage)))))

(event `self.Niagara.OnSystemFinished`
  (params (PSystem :type "NiagaraComponent Object Reference"))
  (`self.K2_DestroyActor`))

(fn `Choose Player`
  (`/Engine/EditorBlueprintResources/ActorMacros.Switch Has Authority`
    (:`Authority`
      (bind _outactors (`GameplayStatics.GetAllActorsOfClass` "/Game/ThirdPerson/Blueprints/BP_ThirdPersonCharacter.BP_ThirdPersonCharacter_C"))
      (bind _returnvalue (`KismetMathLibrary.RandomInteger` (`KismetArrayLibrary.Array_Length` _outactors)))
      (bind _output (`|GetArrayItem` _outactors _returnvalue))
      (if (and (== _output (`self.FollowingPlayer`)) (> _returnvalue 1))
        (`self.Choose Player`)
        (else
          (set `self.FollowingPlayer` _output))))))

(fn `Explode`
  (bind (_returnvalue_x _returnvalue_y _returnvalue_z) (`KismetMathLibrary.BreakVector` (`SceneComponent.K2_GetComponentLocation` (`self.Sphere`))))
  (bind _asbp_enemy_spawner (cast `/Game/Blueprints/BP_EnemySpawner` (`self.SpawnedFromActor`)))
  (`/Game/Blueprints/BP_EnemySpawner.RemoveEnemy` _asbp_enemy_spawner self)
  (`|SpawnActorFromClass` "/Game/StarterContent/Blueprints/Blueprint_Effect_Explosion.Blueprint_Effect_Explosion_C" (`KismetMathLibrary.MakeTransform` (`KismetMathLibrary.MakeVector` _returnvalue_x _returnvalue_y (- _returnvalue_z 500.0))) "Undefined" "MultiplyWithRoot" null null)
  (for _array_element (`PrimitiveComponent.GetOverlappingActors` (`self.ExplosionRadius`) "BP_Enemy_C")
    (bind _asbp_enemy (cast `/Game/Blueprints/BP_Enemy` _array_element))
    (if (not (== self _asbp_enemy))
      (set `/Game/Blueprints/BP_Enemy.HasToExplode` true _asbp_enemy)))
  (`self.K2_DestroyActor`))

(fn `OnRep_ExplodeDamage`)

(fn `OnRep_Health`
  (if (< (`self.Health`) 1)
    (`self.Explode`)))

(fn `UserConstructionScript`)