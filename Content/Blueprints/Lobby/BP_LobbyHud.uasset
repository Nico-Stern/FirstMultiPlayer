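; Lobby HUD Blueprint that creates the lobby UI and limits the start button to the server.
; On BeginPlay it creates WBP_UI for player controller 0, adds it to the viewport and stores the reference.
; An IsServer check shows the start button and mouse cursor on the server, and hides both on other machines.
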(event `self.ReceiveBeginPlay`
  (bind _returnvalue (`GameplayStatics.GetPlayerController` 0))
  (bind _returnvalue_2 (`|CreateWidget` "/Game/Blueprints/Lobby/WBP_UI.WBP_UI_C" (`GameplayStatics.GetPlayerController` 0)))
  (`UserWidget.AddToViewport` _returnvalue_2 0)
  (set `self.UI` _returnvalue_2)
  (if (`KismetSystemLibrary.IsServer`)
    (bind _btn_start (`/Game/Blueprints/Lobby/WBP_UI.btn_Start` _returnvalue_2))
    (set `Widget.Visibility` "Visible" _btn_start)
    (set `PlayerController.bShowMouseCursor` true _returnvalue)
    (else
      (set `Widget.Visibility` "Hidden" _btn_start)
      (set `PlayerController.bShowMouseCursor` false _returnvalue))))

(fn `UserConstructionScript`)