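; BP_Door is a door that opens only while every pressure plate (BP_DruckPlatte) in its Button array is pressed.
; On Tick, the authority side loops through the plates, sets CanDoorBeOpen, stops at the first unpressed one and prints the state as debug text.
; The door's Cube then snaps to a fixed low Z when open, or back to the height cached at BeginPlay when closed, without interpolation.
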(event `self.ReceiveBeginPlay`
  (bind (_returnvalue_x _returnvalue_y _returnvalue_z) (`KismetMathLibrary.BreakVector` (`SceneComponent.K2_GetComponentLocation` (`self.Cube`))))
  (set `self.standarthöhe` _returnvalue_z))

(event `self.ReceiveTick`
  (params (DeltaSeconds :type "Float (single-precision)"))
  (bind _cube (`self.Cube`))
  (bind (_returnvalue_x _returnvalue_y) (`KismetMathLibrary.BreakVector` (`SceneComponent.K2_GetComponentLocation` _cube)))
  (`/Engine/EditorBlueprintResources/ActorMacros.Switch Has Authority`
    (:`Authority`
      (`|ExecutionSequence`
        (:`then_0`
          (for _array_element (`self.Button`)
            (bind _asbp_druck_platte (cast `/Game/Blueprints/BP_DruckPlatte` _array_element))
            (if (`/Game/Blueprints/BP_DruckPlatte.isPressed` _asbp_druck_platte)
              (bind _output_get (set `self.CanDoorBeOpen` true))
              (`KismetSystemLibrary.PrintString` (`KismetStringLibrary.Conv_BoolToString` _output_get) true true (struct :`G` 1.0 :`B` 0.126475 :`A` 1.0))
              (else
                (bind _output_get_2 (set `self.CanDoorBeOpen` false))
                (`KismetSystemLibrary.PrintString` (`KismetStringLibrary.Conv_BoolToString` _output_get_2) true true (struct :`R` 1.0 :`G` 0.248843 :`B` 0.953802 :`A` 1.0))
                (break)))))
        (:`then_1`
          (if (`self.CanDoorBeOpen`)
            (`SceneComponent.K2_SetWorldLocation` _cube (`KismetMathLibrary.MakeVector` _returnvalue_x _returnvalue_y -1000.0) false false)
            (else
              (`SceneComponent.K2_SetWorldLocation` _cube (`KismetMathLibrary.MakeVector` _returnvalue_x _returnvalue_y (`self.standarthöhe`)) false false))))))))

(fn `UserConstructionScript`)