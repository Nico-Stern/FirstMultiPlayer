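; BP_PuzzleCube is a networked rotating puzzle cube that counts as solved when it faces its linked NextCube.
; The server toggles interaction on characters entering or leaving its radius, and Rotate45Degrees adds 45 degrees of yaw through a RepNotify Rotation.
; Despite its name, SendLineTrace traces nothing: each tick it compares rotation to the look-at direction within a tolerance, setting IsPresseed and a green or red material.
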(event `self.ReceiveTick`
  (params (DeltaSeconds :type "Float (single-precision)"))
  (`self.SendLineTrace`))

(event `self.Radius.OnComponentBeginOverlap`
  (params (OverlappedComponent :type "PrimitiveComponent Object Reference") (OtherActor :type "Actor Object Reference") (OtherComp :type "PrimitiveComponent Object Reference") (OtherBodyIndex :type Integer) (bFromSweep :type Boolean) (SweepResult :type "HitResult Structure (by ref)"))
  (`/Engine/EditorBlueprintResources/ActorMacros.Switch Has Authority`
    (:`Authority`
      (bind _asbp_third_person_character (cast `/Game/ThirdPerson/Blueprints/BP_ThirdPersonCharacter` OtherActor))
      (`/Game/ThirdPerson/Blueprints/BP_ThirdPersonCharacter.InteractActivate` _asbp_third_person_character true))))

(event `self.Radius.OnComponentEndOverlap`
  (params (OverlappedComponent :type "PrimitiveComponent Object Reference") (OtherActor :type "Actor Object Reference") (OtherComp :type "PrimitiveComponent Object Reference") (OtherBodyIndex :type Integer))
  (`/Engine/EditorBlueprintResources/ActorMacros.Switch Has Authority`
    (:`Authority`
      (bind _asbp_third_person_character (cast `/Game/ThirdPerson/Blueprints/BP_ThirdPersonCharacter` OtherActor))
      (`/Game/ThirdPerson/Blueprints/BP_ThirdPersonCharacter.InteractActivate` _asbp_third_person_character false))))

(event `Rotate45Degrees`
  (bind (_returnvalue_roll _returnvalue_pitch _returnvalue_yaw) (`KismetMathLibrary.BreakRotator` (`self.K2_GetActorRotation`)))
  (`/Engine/EditorBlueprintResources/ActorMacros.Switch Has Authority`
    (:`Authority`
      (set `self.Rotation` (`KismetMathLibrary.MakeRotator` _returnvalue_roll _returnvalue_pitch (+ _returnvalue_yaw 45.0))))))

(event `SendLineTrace`
  (if (== (`self.K2_GetActorRotation`) (`KismetMathLibrary.FindLookAtRotation` (`self.K2_GetActorLocation`) (`self.K2_GetActorLocation` (`self.NextCube`))) :`ErrorTolerance` 20.0)
    (`PrimitiveComponent.SetMaterial` (`self.Cube`) 0 "/Engine/EngineDebugMaterials/VertexColorViewMode_GreenOnly.VertexColorViewMode_GreenOnly")
    (set `self.IsPresseed` true)
    (else
      (`PrimitiveComponent.SetMaterial` (`self.Cube`) 0 "/Engine/EngineDebugMaterials/VertexColorViewMode_RedOnly.VertexColorViewMode_RedOnly")
      (set `self.IsPresseed` false))))

(fn `OnRep_Rotation`
  (`self.K2_SetActorRotation` (`self.Rotation`)))

(fn `UserConstructionScript`)