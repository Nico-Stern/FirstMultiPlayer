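; Win zone trigger that ends the game with a victory once every BP_ThirdPersonCharacter is inside it.
; On each overlap, the authority compares the count of overlapping characters against all characters in the world and prints a debug "WIN" when all are present.
; It then loops over those characters, pausing the game and showing "Gewonnen" on every BP_GameHUD it finds, all without replicating the UI change to clients.
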(event `self.ReceiveActorBeginOverlap`
  (params (OtherActor :type "Actor Object Reference"))
  (`/Engine/EditorBlueprintResources/ActorMacros.Switch Has Authority`
    (:`Authority`
      (bind _outactors (`GameplayStatics.GetAllActorsOfClass` "/Game/ThirdPerson/Blueprints/BP_ThirdPersonCharacter.BP_ThirdPersonCharacter_C"))
      (if (>= (`KismetArrayLibrary.Array_Length` (`self.GetOverlappingActors` "/Game/ThirdPerson/Blueprints/BP_ThirdPersonCharacter.BP_ThirdPersonCharacter_C")) (`KismetArrayLibrary.Array_Length` _outactors))
        (`KismetSystemLibrary.PrintString` "WIN" true true (struct :`R` 1.0 :`G` 0.074322 :`B` 0.860183 :`A` 1.0) 111.0)
        (for _array_element (`self.GetOverlappingActors` "/Game/ThirdPerson/Blueprints/BP_ThirdPersonCharacter.BP_ThirdPersonCharacter_C")
          (cast `/Game/ThirdPerson/Blueprints/BP_ThirdPersonCharacter` _array_element)
          (`/Engine/EditorBlueprintResources/ActorMacros.Switch Has Authority`
            (:`Authority`
              (`GameplayStatics.SetGamePaused` true)
              (bind _outactors_2 (`GameplayStatics.GetAllActorsOfClass` "/Game/Blueprints/Game/BP_GameHUD.BP_GameHUD_C"))
              (for _array_element_2 _outactors_2
                (bind _tbx_eleminiere (`/Game/Blueprints/Game/WBP_PlayerUI_Ingame.tbx_Eleminiere` (`/Game/Blueprints/Game/BP_GameHUD.PlayerUI` _array_element_2)))
                (set `TextBlock.Text` "Gewonnen" _tbx_eleminiere)
                (`Widget.SetVisibility` _tbx_eleminiere "Visible")
                (`Widget.SetVisibility` (`/Game/Blueprints/Game/WBP_PlayerUI_Ingame.Cvs_GegnerEleminieren` (`/Game/Blueprints/Game/BP_GameHUD.PlayerUI` _array_element_2)) "Visible")))))))))

(fn `UserConstructionScript`)