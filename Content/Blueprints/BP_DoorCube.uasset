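; A puzzle door that opens while the BP_PuzzleCube buttons in its Button array are all pressed.
; On each Tick, only with authority, it scans the array, breaking at the first unpressed button, to update CanDoorBeOpen.
; That flag snaps the Cube down to a fixed low Z or back to the height saved at BeginPlay, without interpolation.
; OpenDoor also sets the flag, but the Tick scan can overwrite it.
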(event `self.ReceiveBeginPlay`
  (bind (_returnvalue_x _returnvalue_y _returnvalue_z) (`KismetMathLibrary.BreakVector` (`SceneComponent.K2_GetComponentLocation` (`self.Cube`))))
  (set `self.standarthöhe` _returnvalue_z))

(event `self.ReceiveTick`
  (params (DeltaSeconds :type "Float (single-precision)"))
  (bind _cube (`self.Cube`))
  (bind (_returnvalue_x _returnvalue_y) (`KismetMathLibrary.BreakVector` (`SceneComponent.K2_GetComponentLocation` _cube)))
  (`/Engine/EditorBlueprintResources/ActorMacros.Switch Has Authority`
    (:`Authority`
      (`|ExecutionSequence`
        (:`then_0`
          (for _array_element (`self.Button`)
            (bind _asbp_puzzle_cube (cast `/Game/Blueprints/BP_PuzzleCube` _array_element))
            (if (`/Game/Blueprints/BP_PuzzleCube.IsPresseed` _asbp_puzzle_cube)
              (set `self.CanDoorBeOpen` true)
              (else
                (set `self.CanDoorBeOpen` false)
                (break)))))
        (:`then_1`
          (if (`self.CanDoorBeOpen`)
            (`SceneComponent.K2_SetWorldLocation` _cube (`KismetMathLibrary.MakeVector` _returnvalue_x _returnvalue_y -1000.0) false false)
            (else
              (`SceneComponent.K2_SetWorldLocation` _cube (`KismetMathLibrary.MakeVector` _returnvalue_x _returnvalue_y (`self.standarthöhe`)) false false))))))))

(fn `OpenDoor`
  (set `self.CanDoorBeOpen` true))

(fn `UserConstructionScript`)