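; Game mode for matches that carries each player's lobby class choice into the game and spawns their characters.
; On controller swap, it copies CharacterClass from BP_LobbyPC to BP_GamePC and registers the controller in AllPlayers.
; After a BeginPlay delay for HUD loading, it replaces each pawn with a BP_ThirdPersonCharacter at the PlayerStart of matching index.
; It then applies class perks: Tank gets higher health, Damage calls SetJumps, Hacker moves faster.
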(event `self.ReceiveBeginPlay`
  ;[1 0 0] Wenn alle hud geladen ist
  (`KismetSystemLibrary.Delay` 3.0)
  (`self.SpawnAllChars`)
  (for (_array_element _array_index) (`self.AllPlayers`)
    (bind _asbp_third_person_character (cast `/Game/ThirdPerson/Blueprints/BP_ThirdPersonCharacter` (`GameplayStatics.GetPlayerPawn` _array_index)))
    (switch `/Game/Blueprints/E_Class` (`/Game/Blueprints/Game/BP_GamePC.CharacterClass` _array_element)
      (:`NewEnumerator1`
        (set `/Game/ThirdPerson/Blueprints/BP_ThirdPersonCharacter.MaxHealth` 220 _asbp_third_person_character)
        (`/Game/ThirdPerson/Blueprints/BP_ThirdPersonCharacter.SetHealth` _asbp_third_person_character))
      (:`NewEnumerator2`
        (`/Game/ThirdPerson/Blueprints/BP_ThirdPersonCharacter.SetJumps` _asbp_third_person_character))
      (:`NewEnumerator3`
        (bind _charactermovement (`Character.CharacterMovement` _asbp_third_person_character))
        (set `CharacterMovementComponent.MaxWalkSpeed` (* (`MovementComponent.GetMaxSpeed` _charactermovement) 1.75) _charactermovement)))))

(event `self.K2_OnSwapPlayerControllers`
  (params (OldPC :type "PlayerController Object Reference") (NewPC :type "PlayerController Object Reference"))
  (bind _asbp_lobby_pc (cast `/Game/Blueprints/Lobby/BP_LobbyPC` OldPC))
  (bind _asbp_game_pc (cast `/Game/Blueprints/Game/BP_GamePC` NewPC))
  (set `/Game/Blueprints/Game/BP_GamePC.CharacterClass` (`/Game/Blueprints/Lobby/BP_LobbyPC.CharacterClass` _asbp_lobby_pc) _asbp_game_pc)
  (`KismetArrayLibrary.Array_AddUnique` (`self.AllPlayers`) _asbp_game_pc))

(event `SpawnAllChars`
  (for (_array_element _array_index) (`self.AllPlayers`)
    (bind _returnvalue (`Controller.K2_GetPawn` _array_element))
    (`/Engine/EditorBlueprintResources/StandardMacros.IsValid` _returnvalue
      (:`Is Valid`
        (`self.K2_DestroyActor` _returnvalue))
      (:`Is Not Valid`
        _))
    (bind _location (`self.FindSpawnPoints` _array_index))
    (bind _returnvalue_2 (`|SpawnActorFromClass` "/Game/ThirdPerson/Blueprints/BP_ThirdPersonCharacter.BP_ThirdPersonCharacter_C" _location "AlwaysSpawn" "MultiplyWithRoot" _array_element null))
    (`Controller.Possess` _array_element _returnvalue_2)))

(fn `FindSpawnPoints`
  (params (index :type Integer))
  (returns (Location :type "Transform Structure"))
  (bind _outactors (`GameplayStatics.GetAllActorsOfClass` "/Script/Engine.PlayerStart"))
  (return (`self.GetTransform` (`|GetArrayItem` _outactors index))))

(fn `UserConstructionScript`)